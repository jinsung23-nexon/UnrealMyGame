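; BP_MgBlockCubeActor is a block cube actor whose material follows a state value.
; SetCubeMaterial switches on the state, applying a basic wall or glass material to the Cube's first slot for the first two states.
; The third state selects a checkered ceramic tile and calls SetMaterialPiled, defined outside this file, instead of setting the Cube material directly.
; Event graph and construction script are empty.
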(event EventBeginPlay)

(event EventActorBeginOverlap
  (params (OtherActor :type Actor%20Object%20Reference)))

(event EventTick
  (params (DeltaSeconds :type Float%20%28single-precision%29)))

(fn ConstructionScript)

(fn SetCubeMaterial
  (params (NewState :type String))
  (switch int (Math|Conversions|ToInteger(Byte) NewState)
    (:Default
      (return))
    (:0
      (LocalVariables|SetNewMaterial "/Game/MobileStarterContent/Materials/M_Basic_Wall.M_Basic_Wall")
      (Rendering|Material|SetMaterial (Variables|Default|GetCube) 0 (LocalVariables|GetNewMaterial) :!label _label))
    (:1
      (LocalVariables|SetNewMaterial "/Game/MobileStarterContent/Materials/M_Glass.M_Glass")
      (goto _label))
    (:2
      (LocalVariables|SetNewMaterial "/Game/MobileStarterContent/Materials/M_Ceramic_Tile_Checker.M_Ceramic_Tile_Checker")
      (Class|MgBlockCubeActor|SetMaterialPiled)))
  (return))