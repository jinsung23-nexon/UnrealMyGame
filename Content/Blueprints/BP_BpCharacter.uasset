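; BP_BpCharacter is the player input Blueprint for a Tetris game, forwarding key presses to TetrisManager.
; Arrow keys and WASD share a MoveBlock helper that turns X/Y steps into an integer vector with zero Z.
; Other keys rotate the block by index, drop it, rotate the camera, or trigger game init, block creation and camera init.
; Q and E both call RotateCamera with the same false argument.
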(event `self.ReceiveBeginPlay`)

(event `self.ReceiveActorBeginOverlap`
  (params (OtherActor :type "Actor Object Reference")))

(event `self.ReceiveTick`
  (params (DeltaSeconds :type "Float (single-precision)")))

(event `Key|Up`
  (params (Key :type "Key Structure" :default "AnyKey"))
  (:`Pressed`
    (`self.MoveBlock` 1 :!label _label)))

(event `Key|Down`
  (params (Key :type "Key Structure" :default "AnyKey"))
  (:`Pressed`
    (`self.MoveBlock` -1 :!label _label_2)))

(event `Key|Left`
  (params (Key :type "Key Structure" :default "AnyKey"))
  (:`Pressed`
    (`self.MoveBlock` 0 -1 :!label _label_3)))

(event `Key|Right`
  (params (Key :type "Key Structure" :default "AnyKey"))
  (:`Pressed`
    (`self.MoveBlock` 0 1 :!label _label_4)))

(event `Key|W`
  (params (Key :type "Key Structure" :default "AnyKey"))
  (:`Pressed`
    (goto _label)))

(event `Key|S`
  (params (Key :type "Key Structure" :default "AnyKey"))
  (:`Pressed`
    (goto _label_2)))

(event `Key|A`
  (params (Key :type "Key Structure" :default "AnyKey"))
  (:`Pressed`
    (goto _label_3)))

(event `Key|D`
  (params (Key :type "Key Structure" :default "AnyKey"))
  (:`Pressed`
    (goto _label_4)))

(event `Key|Z`
  (params (Key :type "Key Structure" :default "AnyKey"))
  (:`Pressed`
    (`/Game/Blueprints/BP_BpTetrisManager.RotateBlock` (`self.TetrisManager`) 0)))

(event `Key|X`
  (params (Key :type "Key Structure" :default "AnyKey"))
  (:`Pressed`
    (`/Game/Blueprints/BP_BpTetrisManager.RotateBlock` (`self.TetrisManager`) 1)))

(event `Key|C`
  (params (Key :type "Key Structure" :default "AnyKey"))
  (:`Pressed`
    (`/Game/Blueprints/BP_BpTetrisManager.RotateBlock` (`self.TetrisManager`) 2)))

(event `Key|Q`
  (params (Key :type "Key Structure" :default "AnyKey"))
  (:`Pressed`
    (`/Game/Blueprints/BP_BpTetrisManager.RotateCamera` (`self.TetrisManager`) false)))

(event `Key|E`
  (params (Key :type "Key Structure" :default "AnyKey"))
  (:`Pressed`
    (`/Game/Blueprints/BP_BpTetrisManager.RotateCamera` (`self.TetrisManager`) false)))

(event `Key|One`
  (params (Key :type "Key Structure" :default "AnyKey"))
  (:`Pressed`
    (`/Game/Blueprints/BP_BpTetrisManager.InitGame` (`self.TetrisManager`))))

(event `Key|Two`
  (params (Key :type "Key Structure" :default "AnyKey"))
  (:`Pressed`
    (`/Game/Blueprints/BP_BpTetrisManager.CreateBlock` (`self.TetrisManager`))))

(event `Key|Three`
  (params (Key :type "Key Structure" :default "AnyKey"))
  (:`Pressed`
    (`/Game/Blueprints/BP_BpTetrisManager.InitCamera` (`self.TetrisManager`))))

(event `Key|SpaceBar`
  (params (Key :type "Key Structure" :default "AnyKey"))
  (:`Pressed`
    (`/Game/Blueprints/BP_BpTetrisManager.DropBlock` (`self.TetrisManager`))))

(fn `MoveBlock`
  (params (MoveX :type Integer) (MoveY :type Integer))
  (`/Game/Blueprints/BP_BpTetrisManager.MoveBlock` (`self.TetrisManager`) (make `/Game/Blueprints/BpIntVector` MoveX MoveY) false))

(fn `UserConstructionScript`)