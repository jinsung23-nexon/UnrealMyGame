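; A block cube actor, apparently one cell of a falling-block puzzle, with falling, predicted and piled states.
; SetState swaps the Cube mesh material to wall, glass or slate to show the current state.
; SetCoordinate takes X, Y and Z but stores nothing, as its variable setters are disconnected.
; The event graph and construction script are empty, so any behavior depends on outside callers.
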(event EventBeginPlay)

(event EventActorBeginOverlap
  (params (OtherActor :type Actor%20Object%20Reference)))

(event EventTick
  (params (DeltaSeconds :type Float%20%28single-precision%29)))

(fn ConstructionScript)

(fn SetCoordinate
  (params (NewX :type Integer) (NewY :type Integer) (NewZ :type Integer))
  (return))

(fn SetState
  (params (NewState :type EBlockCube%20Enum))
  (switch Utilities|FlowControl|Switch|SwitchonEBlockCube NewState
    (:BC_Falling
      (LocalVariables|SetNewMaterial "/Game/MobileStarterContent/Materials/M_Basic_Wall.M_Basic_Wall"))
    (:BC_Predict
      (LocalVariables|SetNewMaterial "/Game/MobileStarterContent/Materials/M_Glass.M_Glass"))
    (:BC_Piled
      (LocalVariables|SetNewMaterial "/Game/MobileStarterContent/Materials/M_Rock_Slate.M_Rock_Slate")))
  (Rendering|Material|SetMaterial (Variables|Default|GetCube) 0 (LocalVariables|GetNewMaterial))
  (return))