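; BP_BpTetrisManager is a manager actor for a Tetris game, handling board dimensions, camera and block data setup.
; The construction script derives map height, cube length and cube scale from the map settings.
; On BeginPlay it positions TetrisCamera at a fixed angled view, blends the player's view to itself, then caches block shapes and cube maximum from LoadBlockData.
; No gameplay loop is implemented in these graphs.
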(event `self.ReceiveBeginPlay`
  (`self.InitCamera`)
  (bind (_blockshapearray _returnvalue) (`MgBpLibrary.LoadBlockData`))
  (set `self.BlockArray` _blockshapearray)
  (set `self.BlockCubeMax` _returnvalue))

(event `self.ReceiveActorBeginOverlap`
  (params (OtherActor :type "Actor Object Reference")))

(event `self.ReceiveTick`
  (params (DeltaSeconds :type "Float (single-precision)")))

(fn `InitCamera`
  (`SceneComponent.K2_SetRelativeLocationAndRotation` (`self.TetrisCamera`) (-200.0 200.0 1200.0) (struct :`Pitch` -50.0) false false)
  (bind _returnvalue (`Controller.CastToPlayerController` (`Pawn.GetController` (`GameplayStatics.GetPlayerCharacter` 0))))
  (`PlayerController.SetViewTargetWithBlend` _returnvalue self "1.0f" "VTBlend_Linear" 0.0 false))

(fn `UserConstructionScript`
  (bind _mapsize (`self.MapSize`))
  (set `self.MapHeight` (+ (`self.StartHeight`) (/ _mapsize 2)))
  (bind _output_get (set `self.CubeLength` (/ (`self.MapLength`) (`KismetMathLibrary.Conv_IntToDouble` _mapsize))))
  (set `self.CubeScale` (/ _output_get "100.f")))